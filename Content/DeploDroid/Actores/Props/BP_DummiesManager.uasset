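; BP_DummiesManager is a prop manager actor that opens the way forward once every dummy in its sector is killed.
; On BeginPlay it records the size of the SectorDummies1 array and binds a counter event to each dummy's BPC_HealthComponent death dispatcher.
; Each death increments the counter; when it equals the dummy count, the linked door (Puerta) is destroyed, with debug prints in Spanish for each outcome.
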(event Custom|DeadDummieCounter
  (Math|Integer|IncrementInt (Variables|Default|GetDeathCounter)
    (:%20%20
      (if (== (Variables|Default|GetEnemyQuantity) (Variables|Default|GetDeathCounter))
        (Actor|DestroyActor (Variables|Default|GetPuerta))
        (Development|PrintString "La puerta se ha destruido" true true "(R=1.000000,G=0.040508,B=0.020612,A=1.000000)" 5.0)
        (else
          (Development|PrintString "Se destruyó un Dummie" true true "(R=1.000000,G=0.040508,B=0.020612,A=1.000000)" 5.0))))))

(event EventBeginPlay
  (bind _sectordummies_1 (Variables|Default|GetSectorDummies_1))
  (Variables|Default|SetEnemyQuantity (Utilities|Array|Length _sectordummies_1))
  (for _array_element _sectordummies_1
    (EventDispatchers|BindEventtoDeadCame (Actor|GetComponentbyClass _array_element "/Game/DeploDroid/Components/BPC_HealthComponent.BPC_HealthComponent_C") (delegate Custom|DeadDummieCounter))))

(fn ConstructionScript)