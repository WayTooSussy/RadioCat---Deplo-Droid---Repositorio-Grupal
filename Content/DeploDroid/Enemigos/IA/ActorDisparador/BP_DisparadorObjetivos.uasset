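; Trigger volume actor that assigns the player as target to a set of enemies.
; When an actor implementing BPI_Jugador begins overlapping, it calls SetearObjetivo with that actor on every entry in the Enemigos array.
; When such an actor leaves the Box component, it calls SetearObjetivo with no target on the same enemies, clearing their objective.
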(event OnComponentEndOverlap(Box)
  (params (OverlappedComponent :type Primitive%20Component%20Object%20Reference) (OtherActor :type Actor%20Object%20Reference) (OtherComp :type Primitive%20Component%20Object%20Reference) (OtherBodyIndex :type Integer))
  (if (Utilities|DoesObjectImplementInterface OtherActor "/Game/DeploDroid/Interfaces/BPI_Jugador.BPI_Jugador_C")
    (for _array_element (Variables|Default|GetEnemigos)
      (Default|SetearObjetivo _array_element))))

(event Collision|EventActorBeginOverlap
  (params (OtherActor :type Actor%20Object%20Reference))
  (if (Utilities|DoesObjectImplementInterface OtherActor "/Game/DeploDroid/Interfaces/BPI_Jugador.BPI_Jugador_C")
    (for _array_element (Variables|Default|GetEnemigos)
      (Default|SetearObjetivo _array_element OtherActor))))

(event EventTick
  (params (DeltaSeconds :type Float%20%28single-precision%29)))

(fn ConstructionScript)