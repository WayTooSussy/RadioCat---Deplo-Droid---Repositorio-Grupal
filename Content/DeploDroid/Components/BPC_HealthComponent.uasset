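; BPC_HealthComponent is a health component that tracks CurrentHealth and takes damage through InflictDamage.
; InflictDamage subtracts the damage, prints Spanish debug messages, and calls DamageDone unless health is exactly zero, where it only prints.
; The clamp node is unconnected, so health can drop below zero, slipping past the equality check and still calling DamageDone.
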(event EventBeginPlay)

(event EventTick
  (params (DeltaSeconds :type Float%20%28single-precision%29)))

(fn InflictDamage
  (params (Daño :type Float%20%28double-precision%29))
  (bind _output_get (Variables|Default|SetCurrentHealth (- (Variables|Default|GetCurrentHealth) Daño)))
  (if (== _output_get 0.0)
    (Development|PrintString "El HP llegó a 0")
    (else
      (Development|PrintString "Se ha perdido HP")
      (Development|PrintString (Utilities|String|ToString(Float) _output_get))
      (Default|CallDamageDone))))