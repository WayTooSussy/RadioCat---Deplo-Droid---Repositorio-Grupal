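; BP_Character is a player character Blueprint that handles movement and sprinting through Enhanced Input.
; On BeginPlay it registers the default input mapping context with its player controller's local player subsystem.
; The move action drives movement along fixed world X and Y axes, independent of camera or control rotation.
; Sprint doubles max walk speed while the action is held and restores it on release.
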(event Input|EnhancedActionEvents|EnhancedInputActionIA_Move
  (params (ActionValue :type Vector%202D%20Structure) (ElapsedSeconds :type Float%20%28double-precision%29) (TriggeredSeconds :type Float%20%28double-precision%29) (InputAction :type Input%20Action%20Object%20Reference :default "/Game/DeploDroid/Character/Input/Input/IA_Move.IA_Move"))
  ;[1 1 1] Movimientos
  (Pawn|Input|AddMovementInput "1.000000,0.000000,0.000000" (.x ActionValue) false)
  (Pawn|Input|AddMovementInput "0.000000,1.000000,0.000000" (.y ActionValue) false))

(event Input|EnhancedActionEvents|EnhancedInputActionIA_Sprint
  (params (ActionValue :type Boolean) (ElapsedSeconds :type Float%20%28double-precision%29) (TriggeredSeconds :type Float%20%28double-precision%29) (InputAction :type Input%20Action%20Object%20Reference :default "/Game/DeploDroid/Character/Input/Input/IA_Sprint.IA_Sprint"))
  ;[1 1 1] Movimientos
  (:Started
    (Variables|/Script/Engine.CharacterMovementComponent|SetMaxWalkSpeed (Variables|Character|GetCharacterMovement) 1.2e+03))
  (:Completed
    (Variables|/Script/Engine.CharacterMovementComponent|SetMaxWalkSpeed (Variables|Character|GetCharacterMovement) 6e+02)))

(event EventBeginPlay
  ;[1 1 1] Controladores
  (bind _asplayer_controller (Utilities|Casting|CastToPlayerController (Pawn|GetController)))
  (Input|AddMappingContext (PlayerController|LocalPlayerSubsystems|GetEnhancedInputLocalPlayerSubsystem _asplayer_controller) "/Game/DeploDroid/Character/Input/IMC_Default.IMC_Default" 0 "(bIgnoreAllPressedKeysUntilRelease=True,bForceImmediately=False,bNotifyUserSettings=False)"))

(fn ConstructionScript
  (|CallParentFunction))